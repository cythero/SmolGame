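; Interaction component that finds the object a player is aiming at, shows its hover prompt and outline, and forwards interact input to it.
; Off dedicated servers, a looping timer box-traces from the camera along view or mouse direction, retracing at half size on multiple hits.
; InteractInterface data validates the hit mesh and drives the HUD text and custom-depth highlight.
; Toggle actors stay highlighted while toggled on.
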(event Custom|Setup
  (params (InteractFocusDistance :type Float%20%28single-precision%29) (TimeBetweenCheckForInteract :type Float%20%28single-precision%29) (TraceSize :type Float%20%28single-precision%29) (InteractionHud :type Interaction%20Hud%20Object%20Reference) (DebugType :type EDrawDebugTrace%20Enum) (TraceFromMousePosition :type Boolean) (Player%20Controller :type Player%20Controller%20Object%20Reference) (TraceChannel :type ETraceTypeQuery%20Enum) (bTraceComplex :type Boolean))
  ;[1 1 1] Setup default variables
  (if (not (Networking|IsDedicatedServer))
    (Utilities|FlowControl|Sequence
      (:then_0
        (Variables|Default|SetTraceChannel TraceChannel)
        (Variables|Default|SetInteractFocusDistance InteractFocusDistance)
        (Variables|Default|SetTraceSize TraceSize)
        (Variables|Default|SetTimeBetweenCheckForInteract TimeBetweenCheckForInteract)
        (Variables|Default|SetbTraceComplex bTraceComplex)
        (Variables|Default|SetInteractionHud InteractionHud)
        (Variables|Default|SetDebugType DebugType)
        (Variables|Default|SetTraceFromMousePosition TraceFromMousePosition)
        (Variables|Default|SetPlayer%20Controller Player%20Controller))
      (:then_1
        ;;[1 1 1] Setup timer
        (Utilities|Time|SetTimerbyFunctionName 0 "Trace" TimeBetweenCheckForInteract true)))))

(fn Trace
  (bind _player_controller (Variables|Default|GetPlayer%20Controller))
  (bind _playercameramanager (Variables|/Script/Engine.PlayerController|GetPlayerCameraManager _player_controller))
  (bind _returnvalue (Transformation|GetActorLocation _playercameramanager))
  ;[1 1 1] Set Start and End
  (LocalVariables|SetStart _returnvalue) ; Set start value for later use
  (LocalVariables|SetEnd (+ _returnvalue (* (select (Variables|Default|GetTraceFromMousePosition) (.WorldDirection (Game|Player|ConvertMouseLocationToWorldSpace (Variables|Default|GetPlayer%20Controller))) (Transformation|GetActorForwardVector _playercameramanager)) (Variables|Default|GetInteractFocusDistance)))) ; Set end value for later use
  ;[1 1 1] Trace for interactable's
  (bind _outhits (Class|KismetSystemLibrary|BoxTraceMulti (LocalVariables|GetStart) (LocalVariables|GetEnd) (Math|Conversions|ToVector(Float) (Variables|Default|GetTraceSize)) "0, 0, 0" (Variables|Default|GetTraceChannel) (Variables|Default|GetbTraceComplex) 0 (Variables|Default|GetDebugType) true))
  ;[1 1 1] Smallen trace if needed
  (if (> (Utilities|Array|Length _outhits) 1) ; If more than one interactable is found, smallen the trace and look for the one closest to the middle of the screen.
    (bind _outhit (Collision|BoxTraceByChannel (LocalVariables|GetStart) (LocalVariables|GetEnd) (Math|Conversions|ToVector(Float) (/ (Variables|Default|GetTraceSize) 2.0)) "0, 0, 0" (Variables|Default|GetTraceChannel) (Variables|Default|GetbTraceComplex) 0 (Variables|Default|GetDebugType))))
  ;[1 1 1] hit something?
  (if (.bBlockingHit (Collision|BreakHitResult (select (> (Utilities|Array|Length _outhits) 1) _outhit (Utilities|Array|Get(acopy) _outhits)))) ; Is there a blocking hit?
    ;[1 1 1] Set HitActor
    (Variables|Default|SethitActor (.HitActor (Collision|BreakHitResult (select (> (Utilities|Array|Length _outhits) 1) _outhit (Utilities|Array|Get(acopy) _outhits)))))
    ;[1 1 1] Is different actor?
    (if (!= (.HitActor (Collision|BreakHitResult (select (> (Utilities|Array|Length _outhits) 1) _outhit (Utilities|Array|Get(acopy) _outhits)))) (Variables|Core|GetInteractActor))
      ;[1 1 1] Set Interface
      (bind _asinteract_interface (Utilities|Casting|CastToInteractInterface (Variables|Default|GethitActor)) ; Does actor have interactinterface?
        (:then
          (bind _output_get (Variables|Default|SetInterface (Utilities|ToObject(Interface) _asinteract_interface)))
          ;[1 1 1] Get data
          (bind _interactcomponents (Class|InteractInterface|GetData(Message) _output_get)) ; Get data from the actor using the interface
          ;[1 1 1] Is hit mesh an interactable
          (bind _containsobject (CallFunction|IsInteractableMesh (.HitComponent (Collision|BreakHitResult (select (> (Utilities|Array|Length _outhits) 1) _outhit (Utilities|Array|Get(acopy) _outhits)))) _interactcomponents))
          ;[1 1 1] Hide old mesh and set the interacting component
          (if _containsobject
            (Variables|Default|SetInteractComponent (.HitComponent (Collision|BreakHitResult (select (> (Utilities|Array|Length _outhits) 1) _outhit (Utilities|Array|Get(acopy) _outhits)))))
            (CallFunction|HideOld)
            ;[1 1 1] Can change the interactable?
            (if (Variables|Default|GetbCanChange)
              ;[1 1 1] Set Interact Actor and close possibility to change
              (Variables|Core|SetInteractActor (Variables|Default|GethitActor))
              (Variables|Default|SetbCanChange false)
              (Utilities|FlowControl|Sequence
                (:then_0
                  ;[1 1 1] Text
                  (bind (_interacthovertext _textcolor _bshowonscreen) (Class|InteractInterface|GetData(Message) (Variables|Default|GetInterface)))
                  ;;[1 1 1] Want to be on screen?
                  (if _bshowonscreen ; Does actor want to be shown on screen?
                    ;;[1 1 1] Set text in umg
                    (Default|Update (Variables|Default|GetInteractionHud) _textcolor (Utilities|Text|ToText(String) _interacthovertext))
                    (else
                      ;;[1 1 1] Hide
                      (Default|Hide (Variables|Default|GetInteractionHud))
                      (CallFunction|HideOld))))
                (:then_1
                  ;[1 1 1] Set Render Depth
                  (bind (_interacthovertext_2 _textcolor_2 _bshowonscreen_2 _blightup _highlightcomponents _outlinecolor) (Class|InteractInterface|GetData(Message) (Variables|Default|GetInterface)))
                  (if _blightup ; Does actor want to be highlighted?
                    (Rendering|Material|SetVectorParameterValue "/Game/Interaction/Materials/Color.Color" "Color" _outlinecolor :!class /Script/Engine.KismetMaterialLibrary)
                    (CallFunction|SetRenderDepth _highlightcomponents)))))))
        (:CastFailed
          ;[1 1 1] Hide
          (Default|Hide (Variables|Default|GetInteractionHud) :!label _label) ; Hide if not in range/view
          (CallFunction|HideOld))))
    (else
      (goto _label))))

(fn HideOld
  ;[1 1 1] Cast to interface
  (bind _asinteract_interface (Utilities|Casting|CastToInteractInterface (Variables|Core|GetInteractActor)) ; Does actor have interactinterface?
    (:then
      (if (Utilities|Array|ContainsItem (Variables|Default|GetToggleItem) (Variables|Core|GetInteractActor))
        (Variables|Default|SetbCanChange true)
        (else
          ;[1 1 1] Get data
          (bind _highlightcomponents (Default|GetData _asinteract_interface))
          ;[1 1 1] remove render depth
          (for _array_element _highlightcomponents
            (Utilities|IsValid _array_element
              (:Is%20Valid
                (bind _asstatic_mesh_component (Utilities|Casting|CastToStaticMeshComponent _array_element)
                  (:then
                    (Rendering|SetRenderCustomDepth _asstatic_mesh_component false))
                  (:CastFailed
                    (bind _asskeletal_mesh_component (Utilities|Casting|CastToSkeletalMeshComponent _array_element))
                    (Rendering|SetRenderCustomDepth _asskeletal_mesh_component false))))))
          (Variables|Default|SetbCanChange true))))
    (:CastFailed
      _))
  (Variables|Core|SetInteractActor 0)
  (return))

(fn Interact
  (params (Key :type Key%20Structure :default "AnyKey") (ActionID :type Integer))
  (bind _interactactor (Variables|Core|GetInteractActor))
  (bind _interactactor_2 (Variables|Core|GetInteractActor))
  (bind _toggleitem (Variables|Default|GetToggleItem))
  (bind _player_controller (Variables|Default|GetPlayer%20Controller))
  ;[1 1 1] Interact
  (Class|InteractInterface|InteractwithObject(Message) _interactactor _player_controller (Pawn|GetControlledPawn _player_controller) Key ActionID (Variables|Default|GetInteractComponent))
  (bind _bistoggleactor (Class|InteractInterface|GetData(Message) _interactactor))
  (if _bistoggleactor
    ;[1 1 1] Add/remove toggle list
    (if (Utilities|Array|ContainsItem (Variables|Default|GetToggleItem) (Variables|Core|GetInteractActor))
      (Utilities|Array|RemoveItem _toggleitem _interactactor_2)
      (else
        (Utilities|Array|Add _toggleitem _interactactor_2)))))

(fn IsInteractableMesh
  (params (Object :type Object%20Object%20Reference) (TargetArray :type Array%20of%20Actor%20Component%20Object%20References))
  ;[1 1 1] Force to false
  (LocalVariables|SetContains false)
  (for _array_element TargetArray
    (Utilities|IsValid _array_element
      (:Is%20Valid
        (bind _asstatic_mesh_component (Utilities|Casting|CastToStaticMeshComponent _array_element)
          (:then
            (if (== Object _asstatic_mesh_component)
              (LocalVariables|SetContains true :!label _label)))
          (:CastFailed
            (bind _asskeletal_mesh_component (Utilities|Casting|CastToSkeletalMeshComponent _array_element))
            (if (== Object _asskeletal_mesh_component)
              (goto _label)))))))
  ;[1 1 1] Return
  (return (LocalVariables|GetContains)))

(fn SetRenderDepth
  (params (Meshes :type Array%20of%20Actor%20Component%20Object%20References))
  (if (> (Utilities|Array|Length Meshes) 0)
    (for _array_element Meshes
      (Utilities|IsValid _array_element
        (:Is%20Valid
          (bind _asstatic_mesh_component (Utilities|Casting|CastToStaticMeshComponent _array_element)
            (:then
              (Rendering|SetRenderCustomDepth _asstatic_mesh_component true))
            (:CastFailed
              (bind _asskeletal_mesh_component (Utilities|Casting|CastToSkeletalMeshComponent _array_element))
              (Rendering|SetRenderCustomDepth _asskeletal_mesh_component true)))))))
  ;[1 1 1] Return
  (return))

(fn GetData
  (bind _array (Utilities|Array|MakeArray 0))
  (return "" "" false false _array "" _array false))