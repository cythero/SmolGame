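; Checkpoint save/load function set that persists player progress to a SaveGame slot and restores player position.
; SaveCheckPoint records location, rotation, variables and reached checkpoint values.
; LoadCheckPoint shares the save object with checkpoint actors and, outside multiplayer, teleports the player to the last checkpoint (linear) or saved location (non-linear), plus offsets.
; Helpers delete or reset the slot, open levels after resetting, and respawn multiplayer players by ID.
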(fn LoadCheckPoint
  (params (MP :type Boolean))
  (bind _outactors (Actor|GetAllActorsOfClass 0))
  (Utilities|IsValid (.Output (Utilities|Array|Get(acopy) _outactors))
    (:Is%20Valid
      (bind _returnvalue (SaveGame|DoesSaveGameExist (Variables|Default|GetCheckPoint%20Slot%20Name (.Item (Utilities|Array|Get(acopy) _outactors)))))
      (if _returnvalue
        (bind _returnvalue_2 (SaveGame|LoadGamefromSlot (Variables|Default|GetCheckPoint%20Slot%20Name (.Item (Utilities|Array|Get(acopy) _outactors)))))
        (bind _ascheck_pointsave (Utilities|Casting|CastTo _returnvalue_2))
        (bind _output_get (LocalVariables|SetSave%20Ref 0 _ascheck_pointsave))
        (LocalVariables|SetPlayerRot (Variables|Default|GetPlayerRotation _output_get))
        (bind _outactors_2 (Actor|GetAllActorsOfClass 0))
        (for (_array_element _array_index) (Variables|Default|GetCheckPointValue _ascheck_pointsave) ; Find the Highest Check Point Value
          (if (> _array_element (Utilities|Array|Get(acopy) (Variables|Default|GetCheckPointValue _ascheck_pointsave) (- _array_index 1)))
            (bind _output_get_2 (Variables|Default|SetLastCheckPointValue _ascheck_pointsave _array_element))))
        (for _array_element_2 _outactors_2
          (Variables|Default|SetSaveGameRef _array_element_2 _ascheck_pointsave)
          (if (and (!= (Utilities|Array|FindItem (Variables|Default|GetCheckPointValue _ascheck_pointsave) (Variables|Default|GetCheckPointValue _array_element_2)) -1) (not MP))
            (CallFunction|ForMultiplayer _array_element_2)
            (if (== (Variables|Default|GetCheckPointValue _array_element_2) _output_get_2)
              (if (Variables|Default|GetLinearOr (.Save%20Ref (LocalVariables|GetSave%20Ref)))
                ;[0.286 1 0.1792] Linear
                (bind _outactors_3 (Actor|GetAllActorsOfClass 0))
                (for (_array_element_3 _array_index_2) _outactors_3
                  (if (== (Variables|Default|GetCheckPointValue _array_element_3) _output_get_2)
                    (LocalVariables|SetPlayerRot (Variables|Default|GetPlayer%20Rotation _array_element_3))))
                (Transformation|SetWorldTransform (Game|GetPlayerCharacter 0) (Math|Transform|MakeTransform (Math|Vector|MakeVector (+ (.X (Math|Vector|BreakVector (Transformation|GetWorldLocation _array_element_2))) (Variables|Default|GetXOffsetToSpawnTo _array_element_2)) (+ (.Y (Math|Vector|BreakVector (Transformation|GetWorldLocation _array_element_2))) (Variables|Default|GetYOffsetToSpawnTo _array_element_2)) (+ (.Z (Math|Vector|BreakVector (Transformation|GetWorldLocation _array_element_2))) (Variables|Default|GetZOffsetToSpawnTo _array_element_2))) (LocalVariables|GetPlayerRot)) false false)
                (Pawn|SetControlRotation (Game|GetPlayerController 0) (LocalVariables|GetPlayerRot))
                (else
                  ;[0.9778 1 0.2394] None-Linear
                  (Transformation|SetWorldTransform (Game|GetPlayerCharacter 0) (Math|Transform|MakeTransform (Math|Vector|MakeVector (+ (.X (Math|Vector|BreakVector (Utilities|Array|Get(acopy) (Variables|Default|GetPlayerLocation (.Save%20Ref (LocalVariables|GetSave%20Ref)))))) (Variables|Default|GetXOffsetToSpawnTo _array_element_2)) (+ (.Y (Math|Vector|BreakVector (Utilities|Array|Get(acopy) (Variables|Default|GetPlayerLocation (.Save%20Ref (LocalVariables|GetSave%20Ref)))))) (Variables|Default|GetYOffsetToSpawnTo _array_element_2)) (+ (.Z (Math|Vector|BreakVector (Utilities|Array|Get(acopy) (Variables|Default|GetPlayerLocation (.Save%20Ref (LocalVariables|GetSave%20Ref)))))) (Variables|Default|GetZOffsetToSpawnTo _array_element_2))) (LocalVariables|GetPlayerRot)) false false)
                  (Pawn|SetControlRotation (Game|GetPlayerController 0) (LocalVariables|GetPlayerRot)))))))
        (else
          ;[1 0.5026 0.9986] CreateSave Object
          (bind _returnvalue_3 (SaveGame|CreateSaveGameObject)) ; Choose Save Game Class Here
          (bind _ascheck_pointsave_2 (Utilities|Casting|CastTo _returnvalue_3))
          (bind _outactors_4 (Actor|GetAllActorsOfClass 0))
          (for _array_element_4 _outactors_4
            (Variables|Default|SetSaveGameRef _array_element_4 _ascheck_pointsave_2)))))))

(fn SaveCheckPoint
  (params (ActorLocation :type Array%20of%20Vectors) (CheckPointValue :type Integer) (CheckPointslotName :type String) (CheckPoint%20Save%20Red :type %20Object%20Reference) (Linear :type Boolean) (PlayerRot :type Rotator) (PlayerVar :type Array%20of%20Floats%20%28single-precision%29))
  (bind _output_get (LocalVariables|SetSaveGameRef 0 CheckPoint%20Save%20Red))
  (Variables|Default|SetLinearOr _output_get Linear)
  (Variables|Default|SetPlayerRotation _output_get PlayerRot)
  (Variables|Default|SetPlayerVariables _output_get PlayerVar)
  (Variables|Default|SetPlayerLocation _output_get ActorLocation)
  (Variables|Default|SetLastCheckPointValue (.SaveGameRef (LocalVariables|GetSaveGameRef)) CheckPointValue)
  (Utilities|Array|AddUnique (Variables|Default|GetCheckPointValue (.SaveGameRef (LocalVariables|GetSaveGameRef))) CheckPointValue)
  (SaveGame|SaveGametoSlot (.SaveGameRef (LocalVariables|GetSaveGameRef)) CheckPointslotName))

(fn DeleteSaveslot
  (bind _outactors (Actor|GetAllActorsOfClass 0))
  (Utilities|IsValid (.Output (Utilities|Array|Get(acopy) _outactors))
    (:Is%20Valid
      (bind _returnvalue (SaveGame|DoesSaveGameExist (Variables|Default|GetCheckPoint%20Slot%20Name (.Item (Utilities|Array|Get(acopy) _outactors)))))
      (if _returnvalue
        (SaveGame|DeleteGameinSlot (Variables|Default|GetCheckPoint%20Slot%20Name (.Item (Utilities|Array|Get(acopy) _outactors))))))))

(fn LoadLevel
  (params (Level :type Byte))
  (CallFunction|ResetSlot)
  (switch Utilities|FlowControl|Switch|Switchon Level
    (:NewEnumerator0
      (Game|OpenLevel(byName) 0 "Level1" false))
    (:NewEnumerator1
      (Game|OpenLevel(byName) 0 "Level2" false))))

(fn ResetSlot
  (bind _outactors (Actor|GetAllActorsOfClass 0))
  (Utilities|IsValid (.Output (Utilities|Array|Get(acopy) _outactors))
    (:Is%20Valid
      (bind _returnvalue (SaveGame|DoesSaveGameExist (Variables|Default|GetCheckPoint%20Slot%20Name (.Item (Utilities|Array|Get(acopy) _outactors)))))
      (if _returnvalue
        (Variables|Default|SetPlayerLocation (Variables|Default|GetSaveGameRef (.Item (Utilities|Array|Get(acopy) _outactors))) (Utilities|Array|MakeArray "0, 0, 0"))
        (Utilities|Array|Clear (Variables|Default|GetCheckPointValue (Variables|Default|GetSaveGameRef (.Item (Utilities|Array|Get(acopy) _outactors)))))
        (Variables|Default|SetLastCheckPointValue (Variables|Default|GetSaveGameRef (.Item (Utilities|Array|Get(acopy) _outactors))) -1)
        (Utilities|Array|Clear (Variables|Default|GetPlayerVariables (Variables|Default|GetSaveGameRef (.Item (Utilities|Array|Get(acopy) _outactors)))))
        (SaveGame|SaveGametoSlot (Variables|Default|GetSaveGameRef (.Item (Utilities|Array|Get(acopy) _outactors))) (Variables|Default|GetCheckPoint%20Slot%20Name (.Item (Utilities|Array|Get(acopy) _outactors))))))))

(fn Respawn
  (params (ID :type Integer))
  ;[1 1 1] Multiplayer Respawn
  (bind _outactors (Actor|GetAllActorsOfClass 0))
  (bind _outactors_2 (Actor|GetAllActorsOfClass 0))
  (for _array_element _outactors_2
    (if (== (Variables|Default|GetPlayer%20ID _array_element) ID)
      (Transformation|SetActorTransform (Pawn|GetControlledPawn _array_element) (Math|Transform|MakeTransform (Utilities|Array|Get(acopy) (Variables|Default|GetPlayerLocation (Variables|Default|GetSaveGameRef (.Item (Utilities|Array|Get(acopy) _outactors)))) ID) (Variables|Default|GetPlayerRotation (Variables|Default|GetSaveGameRef (.Item (Utilities|Array|Get(acopy) _outactors))))))
      (Pawn|SetControlRotation (Game|GetPlayerController 0) (Variables|Default|GetPlayerRotation (Variables|Default|GetSaveGameRef (.Item (Utilities|Array|Get(acopy) _outactors)))))
      (Development|PrintString 0))))