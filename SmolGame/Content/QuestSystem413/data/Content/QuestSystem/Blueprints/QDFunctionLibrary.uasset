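; Blueprint function library for the quest and dialogue system that gives global lookup of its quest, dialogue and utility manager actors.
; Each function gets all actors of the manager class, succeeds only if exactly one exists, and prints an error otherwise.
; It returns a Success flag with the first actor found.
; The quest manager lookup is noted as a fallback for places where the FindQuestManager macro is unavailable, such as UMG.
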(fn GetQuestManager
  ;[1 1 1] Use this function only when you can't use macro (FindQuestManager). For example in UMG
  (bind _outactors (Actor|GetAllActorsOfClass 0 "/Game/QuestSystem/Blueprints/QuestManager.QuestManager_C"))
  (if (== (Utilities|Array|Length _outactors) 1)
    _
    (else
      (Development|PrintString 0 "Could not find single quest manager!" true true "(R=1.000000,G=0.000000,B=0.000000,A=1.000000)")))
  (return (== (Utilities|Array|Length _outactors) 1) (Utilities|Array|Get(acopy) _outactors)))

(fn GetDialogueManager
  (bind _outactors (Actor|GetAllActorsOfClass 0 "/Game/QuestSystem/Blueprints/DialogueManager.DialogueManager_C"))
  (if (== (Utilities|Array|Length _outactors) 1)
    _
    (else
      (Development|PrintString 0 "Could not find single dialogue manager! (QDFunctionLibrary)" true true "(R=1.000000,G=0.000000,B=0.000000,A=1.000000)")
      (Development|PrintString 0 (Utilities|String|ToString(Integer) (Utilities|Array|Length _outactors)) true true "(R=1.000000,G=0.000000,B=0.000000,A=1.000000)")))
  (return (== (Utilities|Array|Length _outactors) 1) (Utilities|Array|Get(acopy) _outactors)))

(fn GetUtilityManager
  (bind _outactors (Actor|GetAllActorsOfClass 0 "/Game/QuestSystem/Blueprints/QDUtilityManager.QDUtilityManager_C"))
  (if (== (Utilities|Array|Length _outactors) 1)
    _
    (else
      (Development|PrintString 0 "Could not find single utility manager!" true true "(R=1.000000,G=0.000000,B=0.000000,A=1.000000)")))
  (return (== (Utilities|Array|Length _outactors) 1) (Utilities|Array|Get(acopy) _outactors)))