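; Quest helper actor that spawns a configurable actor class inside a box volume while a chosen quest or quest node is in a target state.
; It binds to Quest Manager updates and rechecks that state whenever its quest changes and the spawn limit remains unreached.
; Tick then spawns at random points in the box, spaced by a delay, up to the limit.
; The construction script sizes and positions the box and billboard.
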(event Custom|QuestUpdate
  (params (QuestName :type String) (EventType :type EQuestEventType%20Enum))
  (if (and (Utilities|Enum|Equal(Enum) QuestName (Variables|Default|GetQuestName)) (<= (+ (Variables|Default|GetNumSpawned) 1) (Variables|Default|GetSpawnAmount)))
    (bind _timetospawn_ (CallFunction|CheckifSpawnTime))
    (Variables|Default|SetShouldSpawn? _timetospawn_)))

(event EventBeginPlay
  (bind _questmanager (Utilities|FindQuestManager)
    (:QM%20found
      (EventDispatchers|BindEventtoQuestUpdate _questmanager (delegate Custom|QuestUpdate)))))

(event EventTick
  (params (DeltaSeconds :type Float%20%28single-precision%29))
  (bind _box (Variables|Default|GetBox))
  (if (Math|Boolean|ANDBoolean (Variables|Default|GetShouldSpawn?) (< (Variables|Default|GetNumSpawned) (Variables|Default|GetSpawnAmount)) (> (Utilities|Time|GetGameTimeinSeconds) (+ (Variables|Default|GetLastSpawnTime) (Variables|Default|GetDelayBetweenSpawns))))
    (bind _returnvalue (Game|SpawnActorfromClass (Variables|Default|GetActorToSpawn) (Math|Transform|MakeTransform (Math|Random|RandomPointinBoundingBox (Transformation|GetWorldLocation _box) (Variables|/Script/Engine.BoxComponent|GetBoxExtent _box))) true 0))
    (Variables|Default|SetLastSpawnTime (Utilities|Time|GetGameTimeinSeconds))
    (Variables|Default|SetNumSpawned (+ (Variables|Default|GetNumSpawned) 1))
    (Collision|SetActorEnableCollision _returnvalue true)))

(fn ConstructionScript
  (bind _box (Variables|Default|GetBox))
  (bind _boxextent (Variables|Default|GetBoxExtent))
  (bind _boxlocation (Variables|Default|GetBoxLocation))
  (bind _returnvalue (* _boxextent "0, 0,1.000000"))
  (bind _returnvalue_2 (+ _boxlocation _returnvalue))
  (bind (_x _y _z) (Math|Vector|BreakVector _returnvalue_2))
  (Components|Box|SetBoxExtent _box _boxextent true)
  (Transformation|SetRelativeLocation _box _returnvalue_2 false)
  (Transformation|SetRelativeLocation (Variables|Default|GetBillboard) (Math|Vector|MakeVector _x _y (Math|Float|Max(Float) _z 1e+02)) false))

(fn CheckifSpawnTime
  (bind _questmanager (Utilities|FindQuestManager)
    (:QM%20found
      (Utilities|FlowControl|Sequence
        (:then_0
          (if (Utilities|Enum|NotEqual(Enum) (Variables|Default|GetQuestNode) "")
            (bind (_nodefound _questnode) (Default|GetQuestNode _questmanager (Utilities|MakeNodeReference (Variables|Default|GetQuestName) (Variables|Default|GetQuestNode))))
            (if _nodefound
              (LocalVariables|SetLocal_Result (Utilities|Enum|Equal(Enum) (Variables|Default|GetOnState) (.NodeState (Utilities|Struct|BreakQuestNodeStruct _questnode)))))
            (else
              (bind (_questfound _questindex _quest) (Default|GetQuest _questmanager (Variables|Default|GetQuestName)))
              (if _questfound
                (LocalVariables|SetLocal_Result (Utilities|Enum|Equal(Enum) (.QuestState (Utilities|Struct|BreakQuestStruct _quest)) (Variables|Default|GetOnState)))))))
        (:then_1
          (return (LocalVariables|GetLocal_Result)))))))