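; Quest helper actor that, on overlap while enabled, starts a quest or completes or fails a quest node through the QuestManager.
; Quest updates and load events re-check state, showing and enabling it only for a pending quest or active node.
; A dead time guards against repeated overlaps after node changes.
; The construction script configures text and capsule, and Tick yaws the text toward the player's view.
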(event Custom|QuestUpdate_Event_0
  (params (QuestName :type String) (EventType :type EQuestEventType%20Enum))
  ;[1 1 1] When our quest updates check if our node is available
  (if (Utilities|Enum|Equal(Enum) QuestName (Variables|QuestSetting|GetQuestName))
    (CallFunction|CheckifAvailable)))

(event Custom|CustomEvent_0
  (CallFunction|CheckifAvailable))

(event Custom|LoadedFromSaveGame
  (CallFunction|CheckifAvailable))

(event Collision|EventActorBeginOverlap
  (params (OtherActor :type Actor%20Object%20Reference))
  (if (Variables|Default|GetIsEnabled)
    (bind _questmanager (Utilities|FindQuestManager)
      (:QM%20found
        (Variables|Default|SetQuestManager _questmanager)
        (if (< (+ (Variables|Default|GetLastOverlapTime) (Variables|QuestSetting|GetDeadTime)) (Utilities|Time|GetGameTimeinSeconds))
          (if (Variables|QuestSetting|GetQuestNode?) ; Target is quest or quest node?
            (if (Variables|QuestSetting|GetFail?)
              (bind _success (Default|FailQuestNode (Variables|Default|GetQuestManager) (Utilities|MakeNodeReference (Variables|QuestSetting|GetQuestName) (Variables|QuestSetting|GetQuestNodeName)) false))
              (if _success
                (CallFunction|CheckifAvailable :!label _label)
                (Variables|Default|SetLastOverlapTime (Utilities|Time|GetGameTimeinSeconds)))
              (else
                (bind _success_2 (Default|CompleteQuestNode (Variables|Default|GetQuestManager) (Utilities|MakeNodeReference (Variables|QuestSetting|GetQuestName) (Variables|QuestSetting|GetQuestNodeName)) false))
                (if _success_2
                  (goto _label))))
            (else
              (bind _success_3 (Default|StartQuest (Variables|Default|GetQuestManager) (Variables|QuestSetting|GetQuestName)))
              (if _success_3
                (Rendering|SetVisibility false true))))
          (else
            (Development|PrintString "multiple overlaps (QH_OnTouch)")))))))

(event EventBeginPlay
  ;[1 1 1] By default helper is hidden. It is shown only when its quest node is active
  (Rendering|SetVisibility false true)
  (bind _questmanager (Utilities|FindQuestManager)
    (:QM%20found
      (EventDispatchers|AssignQuestUpdate _questmanager (delegate Custom|QuestUpdate_Event_0))
      (EventDispatchers|BindEventtoQuestLoadedfromSavedArray _questmanager (delegate Custom|LoadedFromSaveGame))
      (EventDispatchers|BindEventtoQuestLoadedfromTable _questmanager (delegate Custom|CustomEvent_0)))))

(event EventTick
  (params (DeltaSeconds :type Float%20%28single-precision%29))
  ;[1 1 1] Rotate widget to player
  (Utilities|FlowControl|Sequence
    (:then_0
      (bind _ascharacter (Utilities|Casting|CastToCharacter (Game|Player|GetPlayerPawn 0))
        (:then
          (Variables|Default|SetPlayerCameraRotation (Pawn|GetControlRotation _ascharacter :!class /Script/Engine.Pawn)))
        (:CastFailed
          (bind _asvehicle_blueprint (Utilities|Casting|CastToVehicleBlueprint (Game|Player|GetPlayerPawn 0)))
          (Variables|Default|SetPlayerCameraRotation (Transformation|GetWorldRotation _asvehicle_blueprint)))))
    (:then_1
      (Transformation|SetWorldRotation (Variables|Default|GetTextRender) (Math|Rotator|MakeRotator 0.0 (+ (.Yaw (Class|KismetMathLibrary|BreakRot (Variables|Default|GetPlayerCameraRotation))) 1.8e+02) 0.0) false))))

(fn ConstructionScript
  (bind _textrender (Variables|Default|GetTextRender))
  (bind _capsule (Variables|Default|GetCapsule))
  (bind _capsulehalfheight (Variables|Appearing|GetCapsuleHalfHeight))
  (Rendering|Components|TextRender|SetText _textrender (Variables|Appearing|GetDisplayedText))
  (Rendering|Components|TextRender|SetTextRenderColor _textrender (Math|Conversions|ToColor(LinearColor) (Variables|Appearing|GetTextColor)))
  (Components|Capsule|SetCapsuleSize _capsule (Variables|Appearing|GetCapsuleRadius) _capsulehalfheight true)
  (Transformation|SetRelativeLocation _capsule (Math|Vector|MakeVector 0.0 0.0 (- _capsulehalfheight (Variables|Appearing|GetCapsuleRadius))) false))

(fn CheckifAvailable
  (bind _questmanager (Utilities|FindQuestManager)
    (:QM%20found
      (if (Variables|QuestSetting|GetQuestNode?)
        (bind (_nodefound _questnode) (Default|GetQuestNode _questmanager (Utilities|MakeNodeReference (Variables|QuestSetting|GetQuestName) (Variables|QuestSetting|GetQuestNodeName))))
        (if _nodefound
          (switch Utilities|FlowControl|Switch|SwitchonEQuestNodeState (.NodeState (Utilities|Struct|BreakQuestNodeStruct _questnode))
            (:NewEnumerator0
              (Rendering|SetVisibility true true)
              (Variables|Default|SetIsEnabled true))
            (:NewEnumerator1
              (Rendering|SetVisibility false true :!label _label)
              (Variables|Default|SetIsEnabled false))
            (:NewEnumerator2
              (goto _label))
            (:NewEnumerator3
              (goto _label))
            (:NewEnumerator4
              (goto _label))))
        (else
          (bind (_questfound _questindex _quest) (Default|GetQuest _questmanager (Variables|QuestSetting|GetQuestName)))
          (if _questfound
            (switch Utilities|FlowControl|Switch|SwitchonEQuestNodeState (.QuestState (Utilities|Struct|BreakQuestStruct _quest))
              (:NewEnumerator0
                (Rendering|SetVisibility false true :!label _label_2)
                (Variables|Default|SetIsEnabled false))
              (:NewEnumerator1
                (goto _label_2))
              (:NewEnumerator2
                (Rendering|SetVisibility true true)
                (Variables|Default|SetIsEnabled true))
              (:NewEnumerator3
                (goto _label_2))
              (:NewEnumerator4
                (goto _label_2)))))))))