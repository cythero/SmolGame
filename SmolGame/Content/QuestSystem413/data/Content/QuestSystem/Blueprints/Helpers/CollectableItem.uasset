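; Collectable quest item actor that, on its ItemCollected event, updates a quest, adds its name to the player's inventory and destroys itself.
; HandleQuest finds the quest manager, then either starts a quest or completes or fails a quest node, depending on its flags.
; The construction script configures label and capsule.
; Pawn overlap can reveal the label, which Tick yaws toward the camera; the end-overlap hide is disabled by a false branch.
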(event Custom|ItemCollected
  (Utilities|FlowControl|Sequence
    (:then_0
      (|HandleQuest))
    (:then_1
      (|AddToInventory))
    (:then_2
      (Actor|DestroyActor))))

(event EventActorBeginOverlap
  (params (OtherActor :type Actor%20Object%20Reference))
  (if (Variables|Default|GetDisplayNameText)
    (Utilities|Casting|CastToPawn OtherActor)
    (Rendering|SetVisibility (Variables|Default|GetTextRender) true false)))

(event EventActorEndOverlap
  (params (OtherActor :type Actor%20Object%20Reference))
  (if false
    (Utilities|Casting|CastToPawn OtherActor)
    (Rendering|SetVisibility (Variables|Default|GetTextRender) false false)))

(event EventTick
  (params (DeltaSeconds :type Float%20%28single-precision%29))
  ;[1 1 1] Rotate widget to player
  (Utilities|FlowControl|Sequence
    (:then_0
      (bind _ascharacter (Utilities|Casting|CastToCharacter (Game|Player|GetPlayerPawn 0))
        (:then
          (Variables|Default|SetPlayerCameraRotation (Pawn|GetControlRotation _ascharacter :!class /Script/Engine.Pawn)))
        (:CastFailed
          (Development|PrintString "cast failed inside of collectableitem" true true "(R=1.000000,G=0.000000,B=0.000000,A=1.000000)"))))
    (:then_1
      (Transformation|SetWorldRotation (Variables|Default|GetTextRender) (Math|Rotator|MakeRotator 0.0 (+ (.Yaw (Class|KismetMathLibrary|BreakRot (Variables|Default|GetPlayerCameraRotation))) 1.8e+02) 0.0) false))))

(event EventBeginPlay
  (Rendering|SetVisibility (Variables|Default|GetTextRender) false false))

(fn ConstructionScript
  (bind _textrender (Variables|Default|GetTextRender))
  (bind _capsule (Variables|Default|GetCapsule))
  (bind _capsulehalfheight (Variables|Appearence|GetCapsuleHalfHeight))
  (Rendering|Components|TextRender|SetText _textrender (Variables|Appearence|GetDisplayedText))
  (Rendering|Components|TextRender|SetTextRenderColor _textrender (Math|Conversions|ToColor(LinearColor) (Variables|Appearence|GetTextColor)))
  (Components|Capsule|SetCapsuleSize _capsule (Variables|Appearence|GetCapsuleRadius) _capsulehalfheight true)
  (Transformation|SetRelativeLocation _capsule (Math|Vector|MakeVector 0.0 0.0 (- _capsulehalfheight (Variables|Appearence|GetCapsuleRadius))) false))