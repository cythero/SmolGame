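; DialogueCharacter is a quest system helper actor for an NPC with dialogue and a displayed name.
; The construction script sizes and offsets the dialogue collision capsule, sets the name text, and copies dialogue, bark, voice, montage and radius settings into DialogueNPCComp.
; Each tick turns the name text to face opposite the player's control yaw.
; StartDialogue finds the dialogue manager and starts its configured dialogue in the foreground.
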(event EventTick
  (params (DeltaSeconds :type Float%20%28single-precision%29))
  (Utilities|FlowControl|Sequence
    (:then_0
      (bind _ascharacter (Utilities|Casting|CastToCharacter (Game|Player|GetPlayerPawn 0))
        (:then
          (Variables|Default|SetPlayerCamRot (Pawn|GetControlRotation _ascharacter :!class /Script/Engine.Pawn)))
        (:CastFailed
          (Development|PrintString "cast failed inside of DialogueCharacter" true true "(R=1.000000,G=0.000000,B=0.000000,A=1.000000)"))))
    (:then_1
      (Transformation|SetWorldRotation (Variables|Default|GetCharacterName) (Math|Rotator|MakeRotator 0.0 (+ (.Yaw (Class|KismetMathLibrary|BreakRot (Variables|Default|GetPlayerCamRot))) 1.8e+02) 0.0) false))))

(fn ConstructionScript
  (bind _dialoguenpccomp (Variables|Default|GetDialogueNPCComp))
  (Utilities|FlowControl|Sequence
    (:then_0
      (|ResizeCapsule))
    (:then_1
      (Rendering|Components|TextRender|SetText (Variables|Default|GetCharacterName) (Utilities|Text|ToText(String) (Variables|Default|GetDisplayedName)))
      (Variables|/Game/QuestSystem/Blueprints/Helpers/DialogueNPCComp.DialogueNPCComp_C|SetDialogueName _dialoguenpccomp (Variables|Default|GetDialogueName))
      (Variables|/Game/QuestSystem/Blueprints/Helpers/DialogueNPCComp.DialogueNPCComp_C|SetTechName _dialoguenpccomp (Variables|Default|GetTechName))
      (Variables|/Game/QuestSystem/Blueprints/Helpers/DialogueNPCComp.DialogueNPCComp_C|SetDisplayedName _dialoguenpccomp (Variables|Default|GetDisplayedName))
      (Variables|/Game/QuestSystem/Blueprints/Helpers/DialogueNPCComp.DialogueNPCComp_C|SetCanBark _dialoguenpccomp (Variables|Default|GetCanBark))
      (Variables|/Game/QuestSystem/Blueprints/Helpers/DialogueNPCComp.DialogueNPCComp_C|SetBarkDialogueName _dialoguenpccomp (Variables|Default|GetBarkDialogue))
      (Variables|/Game/QuestSystem/Blueprints/Helpers/DialogueNPCComp.DialogueNPCComp_C|SetVoiceOverCue _dialoguenpccomp (Variables|Default|GetVoiceOver))
      (Variables|/Game/QuestSystem/Blueprints/Helpers/DialogueNPCComp.DialogueNPCComp_C|SetAnimMontage _dialoguenpccomp (Variables|Default|GetAnimMontage))
      (Variables|/Game/QuestSystem/Blueprints/Helpers/DialogueNPCComp.DialogueNPCComp_C|SetTalkRadius _dialoguenpccomp (Variables|Default|GetTalkRadius))
      (Variables|/Game/QuestSystem/Blueprints/Helpers/DialogueNPCComp.DialogueNPCComp_C|SetBarkRadius _dialoguenpccomp (Variables|Default|GetBarkRadius))
      (Variables|/Game/QuestSystem/Blueprints/Helpers/DialogueNPCComp.DialogueNPCComp_C|SetStopRadius _dialoguenpccomp (Variables|Default|GetStopRadius))
      (Variables|/Game/QuestSystem/Blueprints/Helpers/DialogueNPCComp.DialogueNPCComp_C|SetSilencePeriod _dialoguenpccomp (Variables|Default|GetSilencePeriod)))))

(fn StartDialogue
  (bind _dialogue_manager (Utilities|FindDialogueManager)
    (:DM%20found
      (Default|StartDialogue _dialogue_manager (Variables|Default|GetDialogueName) false))))