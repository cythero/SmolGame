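; Actor component that hooks its owning NPC into the quest system's dialogue manager.
; After a short delay on initialization it registers the owner and itself, then binds the owner's overlap events.
; Begin and end overlaps are reported to the manager as player overlaps, without checking the other actor.
; WantToBark rate-limits barks, returning true and resetting LastTimeTalked only once SilencePeriod has elapsed.
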(event Custom|OnActorBeginOverlap_Event_0
  (params (OtherActor :type Actor%20Object%20Reference))
  (bind (_success _dialogue_manager) (CallFunction|GetDialogueManager))
  (if _success
    (Default|NPCBeginOverlapPlayer _dialogue_manager self)))

(event Custom|OnActorEndOverlap_Event_0
  (params (OtherActor :type Actor%20Object%20Reference))
  (bind (_success _dialogue_manager) (CallFunction|GetDialogueManager))
  (if _success
    (Default|NPCEndOverlapPlayer _dialogue_manager self)))

(event EventTick
  (params (DeltaSeconds :type Float%20%28single-precision%29)))

(event EventInitializeComponent
  (bind _returnvalue (Components|GetOwner))
  (Utilities|FlowControl|Delay 0.2)
  (bind (_success _dialogue_manager) (CallFunction|GetDialogueManager))
  (if _success
    (Default|RegisterNPC _dialogue_manager _returnvalue self)
    (EventDispatchers|AssignOnActorBeginOverlap _returnvalue (delegate Custom|OnActorBeginOverlap_Event_0))
    (EventDispatchers|AssignOnActorEndOverlap (Components|GetOwner) (delegate Custom|OnActorEndOverlap_Event_0))))

(fn WanttoBark
  (bind _returnvalue (Utilities|Time|GetGameTimeinSeconds))
  (Math|Float|CompareFloat (+ (Variables|Default|GetLastTimeTalked) (Variables|Default|GetSilencePeriod)) _returnvalue
    (:>
      (LocalVariables|SetLocal_Result false :!label _label))
    (:==
      (goto _label))
    (:<
      (Variables|Default|SetLastTimeTalked _returnvalue)
      (LocalVariables|SetLocal_Result true)))
  (return (LocalVariables|GetLocal_Result)))